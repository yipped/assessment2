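; Mirror actor Blueprint that intensifies its material's vertex animation as the player character gets closer.
; BeginPlay creates a dynamic material instance on the Mirror component and caches the BP_ThirdPersonCharacter player.
; Each Tick sets VertexStrength to one minus the clamped ratio of player distance to MaxDistance.
; That distance is measured from the world origin, not the mirror's own location.
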(event `self.ReceiveBeginPlay`
  (bind _mirror (`self.mirror`))
  ; Creates new dynamic material to reference on startup and get player character to dynamically change material with player position
  (bind _returnvalue (`PrimitiveComponent.CreateDynamicMaterialInstance` _mirror 0 (`PrimitiveComponent.GetMaterial` _mirror 0) "None"))
  (set `self.MirrorDynamicMaterial` _returnvalue)
  (bind _asbp_third_person_character (cast `/Game/ThirdPerson/Blueprints/BP_ThirdPersonCharacter` (`GameplayStatics.GetPlayerCharacter` 0)))
  (set `self.As BP Third Person Character` _asbp_third_person_character))

(event `self.ReceiveTick`
  (params (DeltaSeconds :type "Float (single-precision)"))
  ; As the player gets closer to the material the intensity of the vertex animation gets greater
  (`MaterialInstanceDynamic.SetScalarParameterValue` (`self.MirrorDynamicMaterial`) "VertexStrength" (- (`self.1`) (`KismetMathLibrary.FClamp` (`KismetMathLibrary.SafeDivide` (`KismetMathLibrary.Vector_Distance` (`self.K2_GetActorLocation` (`self.As BP Third Person Character`))) (`self.MaxDistance`))))))

(fn `UserConstructionScript`)