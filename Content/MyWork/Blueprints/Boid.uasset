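; Flocking boid actor that steers itself each Tick using separation, alignment and cohesion.
; Sphere overlap events maintain NearbyBoids from Boid_old actors, but add and remove inside loops over that array, so an empty list never gains entries.
; Three custom events turn neighbour positions and velocities into weighted forces.
; Move1 sums these into a speed-capped Velocity and offsets the location without sweep or delta-time scaling.
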(event `self.Sphere.OnComponentEndOverlap`
  (params (OverlappedComponent :type "PrimitiveComponent Object Reference") (OtherActor :type "Actor Object Reference") (OtherComp :type "PrimitiveComponent Object Reference") (OtherBodyIndex :type Integer))
  ; Adding and removing other boid objects from array through collision sphere
  (bind _asboid (cast `/Game/MyWork/Blueprints/Boid_old` OtherActor))
  (for _ (`self.NearbyBoids`)
    (`KismetArrayLibrary.Array_RemoveItem` (`self.NearbyBoids`) _asboid)))

(event `self.Sphere.OnComponentBeginOverlap`
  (params (OverlappedComponent :type "PrimitiveComponent Object Reference") (OtherActor :type "Actor Object Reference") (OtherComp :type "PrimitiveComponent Object Reference") (OtherBodyIndex :type Integer) (bFromSweep :type Boolean) (SweepResult :type "HitResult Structure (by ref)"))
  (bind _nearbyboids (`self.NearbyBoids`))
  ; Adding and removing other boid objects from array through collision sphere
  (bind _asboid (cast `/Game/MyWork/Blueprints/Boid_old` OtherActor))
  (for _ (`self.NearbyBoids`)
    (`KismetArrayLibrary.Array_Add` _nearbyboids _asboid)
    (`KismetSystemLibrary.PrintString` (`KismetStringLibrary.Conv_IntToString` (`KismetArrayLibrary.Array_Length` _nearbyboids)))))

(event `self.ReceiveTick`
  (params (DeltaSeconds :type "Float (single-precision)"))
  ; Main
  (`self.Separation1`)
  (`self.Alignment1`)
  (`self.Cohesion1`)
  (`self.Move1`))

(event `Separation1`
  ; Separation
  (set `self.Sum` (0.0 0.0 0.0))
  (for _array_element (`self.NearbyBoids`)
    (bind _returnvalue (- (`self.K2_GetActorLocation`) (`self.K2_GetActorLocation` _array_element)))
    (set `self.Sum` (+ (/ (`KismetMathLibrary.Normal` _returnvalue) (`KismetMathLibrary.FClamp` (`KismetMathLibrary.VSize` _returnvalue) 1.0 0.0)) (`self.Sum`))))
  (set `self.SeparationForce` (* (`KismetMathLibrary.Normal` (`self.Sum`)) (`self.SeparationWeight`))))

(event `Alignment1`
  (bind _nearbyboids (`self.NearbyBoids`))
  ; Alignment
  (set `self.Sum` (0.0 0.0 0.0))
  (set `self.AlignmentForce` (0.0 0.0 0.0))
  (for _array_element _nearbyboids
    (set `self.Sum` (+ (`/Game/MyWork/Blueprints/Boid_old.Velocity` _array_element) (`self.Sum`))))
  (set `self.AlignmentForce` (* (`KismetMathLibrary.Normal` (/ (`self.Sum`) (`KismetArrayLibrary.Array_Length` _nearbyboids))) (`self.AlignmentWeight`))))

(event `Cohesion1`
  ; Cohesion
  (set `self.CohesionForce` (0.0 0.0 0.0))
  (for _ (`self.NearbyBoids`)
    (bind _returnvalue (`GameplayStatics.GetActorArrayAverageLocation` (`self.NearbyBoids`)))
    (bind _output_get (set `self.Center` _returnvalue))
    (set `self.CohesionForce` (* (`self.CohesionWeight`) (`KismetMathLibrary.Normal` (- _output_get (`self.K2_GetActorLocation`)))))))

(event `Move1`
  ; Combining forces
  (set `self.SteeringForce` (+ (`self.SeparationForce`) (`self.AlignmentForce`) (`self.CohesionForce`)))
  (set `self.Velocity` (`KismetMathLibrary.Vector_ClampSizeMax` (+ (`self.Velocity`) (* (`self.SteeringForce`) (`self.SteeringStrength`))) (`self.MaxSpeed`)))
  (`self.K2_SetActorLocation` (+ (`self.K2_GetActorLocation`) (`self.Velocity`))))

(event `Cohesion`)

(event `Alignment`)

(event `Move`)

(fn `Separation`)

(fn `UserConstructionScript`)