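; Cultist is an actor that watches the player and plays an animation when approached.
; On BeginPlay it caches the third person player character, then every Tick snaps its rotation to look at that character using FindLookAtRotation.
; When the player character overlaps its Box trigger, the Cultist skeletal mesh plays CultistAnimation once, without looping.
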(event `self.ReceiveBeginPlay`
  ; Sets third person character control on start
  (bind _asbp_third_person_character (cast `/Game/ThirdPerson/Blueprints/BP_ThirdPersonCharacter` (`GameplayStatics.GetPlayerCharacter` 0)))
  (set `self.As BP Third Person Character` _asbp_third_person_character))

(event `self.ReceiveTick`
  (params (DeltaSeconds :type "Float (single-precision)"))
  ; Rotates model to look at player
  (`self.K2_SetActorRotation` (`KismetMathLibrary.FindLookAtRotation` (`self.K2_GetActorLocation`) (`self.K2_GetActorLocation` (`self.As BP Third Person Character`)))))

(event `self.Box.OnComponentBeginOverlap`
  (params (OverlappedComponent :type "PrimitiveComponent Object Reference") (OtherActor :type "Actor Object Reference") (OtherComp :type "PrimitiveComponent Object Reference") (OtherBodyIndex :type Integer) (bFromSweep :type Boolean) (SweepResult :type "HitResult Structure (by ref)"))
  ; Plays skeletal animation when player enters collision
  (cast `/Game/ThirdPerson/Blueprints/BP_ThirdPersonCharacter` OtherActor)
  (`SkeletalMeshComponent.PlayAnimation` (`self.cultist`) "/Game/MyWork/Models/Cultist/cultistAnimation.cultistAnimation" false))

(fn `UserConstructionScript`)