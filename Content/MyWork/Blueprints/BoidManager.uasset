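; BoidManager is a spawner that creates Boid actors in the level when play begins.
; A BeginPlay loop, currently set to a single iteration, spawns each Boid at a random position in an elevated box with a random rotation.
; Each new Boid then receives a small random Velocity vector.
; The manager does nothing after spawning, as its Tick and overlap events are empty.
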(event `self.ReceiveBeginPlay`
  (for _ (range 1)
    (bind _returnvalue (`|SpawnActorFromClass` "/Game/MyWork/Blueprints/Boid.Boid_C" (`KismetMathLibrary.MakeTransform` (`KismetMathLibrary.MakeVector` (`KismetMathLibrary.Conv_IntToDouble` (`KismetMathLibrary.RandomIntegerInRange` -2000 2000)) (`KismetMathLibrary.Conv_IntToDouble` (`KismetMathLibrary.RandomIntegerInRange` -2000 2000)) (`KismetMathLibrary.Conv_IntToDouble` (`KismetMathLibrary.RandomIntegerInRange` 1500 2000))) (`KismetMathLibrary.MakeRotator` (`KismetMathLibrary.Conv_IntToDouble` (`KismetMathLibrary.RandomIntegerInRange` 0 360)) (`KismetMathLibrary.Conv_IntToDouble` (`KismetMathLibrary.RandomIntegerInRange` 0 360)) (`KismetMathLibrary.Conv_IntToDouble` (`KismetMathLibrary.RandomIntegerInRange` 0 360)))) "Undefined" "MultiplyWithRoot" null null))
    (set `/Game/MyWork/Blueprints/Boid.Velocity` (`KismetMathLibrary.MakeVector` (`KismetMathLibrary.Conv_IntToDouble` (`KismetMathLibrary.RandomIntegerInRange` -5 5)) (`KismetMathLibrary.Conv_IntToDouble` (`KismetMathLibrary.RandomIntegerInRange` -5 5)) (`KismetMathLibrary.Conv_IntToDouble` (`KismetMathLibrary.RandomIntegerInRange` -5 5))) _returnvalue)))

(fn `UserConstructionScript`)